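; BP_HookShot is a grappling hook actor that finds a hook point along the player's camera direction and draws the chain to it.
; CalcHookShotHit line-traces for a hit, then capsule-traces from a backed-off point to return a player-sized end location and success flag.
; It sets the Going state; outside Idle, Tick orients the hook and chain, scaling the first link for the remainder and using instanced meshes for whole links.
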(event `self.ReceiveBeginPlay`
  (bind _asbp_player (cast `/Game/_Manager/BP_Player` (`GameplayStatics.GetPlayerCharacter` 0)))
  (set `self.Player Ref` _asbp_player))

(event `self.ReceiveTick`
  (params (DeltaSeconds :type "Float (single-precision)"))
  (bind _hook_states (`self.Hook States`))
  (`|ExecutionSequence`
    (:`then_0`
      (switch `/Game/Grappling_Hook/E_Hookhot_States` _hook_states
        (:`NewEnumerator2`
          (set `self.End Location` (`KismetMathLibrary.VInterpTo_Constant` (`self.End Location`))))))
    (:`then_1`
      (if (`|EnumInequality` _hook_states "NewEnumerator1")
        (`self.Chain Movement`)))))

(fn `Calc HookShot Hit`
  (params (`Shot Distance` :type "Float (double-precision)" :default 2000.0) (`Backoff Distance` :type "Float (double-precision)" :default 200.0))
  (returns (`Hook End Location` :type "Vector Structure") (`Hit Sucess` :type Boolean))
  (locals (`HookShot Distance` :type "Float (double-precision)" :default 100.0) (`Hook Backoff Distance` :type "Float (double-precision)" :default 100.0))
  (bind _returnvalue (`self.K2_GetActorLocation`))
  (bind _player_ref (`self.Player Ref`))
  (bind _array (`|MakeArray` _player_ref :!type "Actor Object Reference"))
  (bind _capsulecomponent (`Character.CapsuleComponent` (`self.Player Ref`)))
  (set `local.HookShot Distance` `Shot Distance`)
  (set `local.Hook Backoff Distance` `Backoff Distance`)
  (bind (_outhit _returnvalue_2) (`KismetSystemLibrary.LineTraceSingle` _returnvalue (+ _returnvalue (* (`SceneComponent.GetForwardVector` (`/Game/_Manager/BP_Player.Camera` _player_ref)) (`local.HookShot Distance`))) "TraceTypeQuery3" false _array "ForDuration" true (struct :`R` 1.0 :`A` 1.0) (struct :`G` 1.0 :`A` 1.0) 2.5))
  (if _returnvalue_2
    (bind (_bblockinghit _binitialoverlap _time _distance _location _impactpoint _normal _impactnormal _physmat _hitactor _hitcomponent _hitbonename _bonename _hititem _elementindex _faceindex _tracestart _traceend) (`GameplayStatics.BreakHitResult` _outhit))
    (set `self.End Location` _location)
    (`self.HandleSetHookShotStates` "NewEnumerator2")
    (bind (_outhit_2 _returnvalue_3) (`KismetSystemLibrary.CapsuleTraceSingle` (- _location (* (`KismetMathLibrary.GetDirectionUnitVector` _tracestart _traceend) (`local.Hook Backoff Distance`))) _location (`CapsuleComponent.GetScaledCapsuleRadius` _capsulecomponent) (`CapsuleComponent.GetScaledCapsuleHalfHeight` _capsulecomponent) "TraceTypeQuery1" false _array "ForDuration" true (struct :`R` 1.0 :`A` 1.0) (struct :`G` 1.0 :`A` 1.0) 2.5))
    (if _returnvalue_3
      (bind (_bblockinghit_2 _binitialoverlap_2 _time_2 _distance_2 _location_2 _impactpoint_2 _normal_2 _impactnormal_2 _physmat_2 _hitactor_2 _hitcomponent_2 _hitbonename_2 _bonename_2 _hititem_2 _elementindex_2 _faceindex_2 _tracestart_2 _traceend_2) (`GameplayStatics.BreakHitResult` _outhit_2))
      (return _location_2 true)
      (else
        (return _traceend_2 true)))
    (else
      (set `self.End Location` _traceend)
      (`self.HandleSetHookShotStates` "NewEnumerator2")
      (return (0.0 0.0 0.0) false))))

(fn `Chain Movement`
  (bind _returnvalue (`self.K2_GetActorLocation`))
  (bind _firstchain (`self.FirstChain`))
  (bind _end_location (`self.End Location`))
  (bind _end_location_2 (`self.End Location`))
  (bind _chain_length (`self.Chain Length`))
  (bind _returnvalue_2 (`InstancedStaticMeshComponent.GetInstanceCount` (`self.Instanced Chains`)))
  (bind _returnvalue_3 (`KismetMathLibrary.GetDirectionUnitVector` _returnvalue _end_location_2))
  (bind (_remainder _returnvalue_4) (`KismetMathLibrary.FMod` (`KismetMathLibrary.Vector_Distance` _returnvalue _end_location_2) (`self.Chain Length`)))
  (bind _returnvalue_5 (`KismetMathLibrary.Conv_VectorToRotator` (`KismetMathLibrary.GetDirectionUnitVector` (`self.K2_GetActorLocation`) _end_location)))
  (bind _returnvalue_6 (- _returnvalue_4 1))
  (`|ExecutionSequence`
    (:`then_0`
      ; Hook
      (`SceneComponent.K2_SetWorldLocationAndRotation` (`self.Hook`) _end_location _returnvalue_5 false false))
    (:`then_1`
      ; First Chain
      (`SceneComponent.K2_SetWorldRotation` _firstchain _returnvalue_5 false false)
      (`SceneComponent.SetRelativeScale3D` _firstchain (`KismetMathLibrary.MakeVector` (/ (`KismetMathLibrary.FMod` (`KismetMathLibrary.Vector_Distance` (`self.K2_GetActorLocation`) (`self.End Location`)) _chain_length) _chain_length) 1.0 1.0)))
    (:`then_2`
      ; Chain Instances
      (if (> _returnvalue_4 0)
        (`SceneComponent.K2_SetWorldLocationAndRotation` (`self.Instanced Chains`) (+ _returnvalue (* _returnvalue_3 _remainder)) (`KismetMathLibrary.Conv_VectorToRotator` _returnvalue_3) false false)
        (if (> _returnvalue_4 _returnvalue_2)
          (for _index (range _returnvalue_2 (+ _returnvalue_6 1))
            (`InstancedStaticMeshComponent.AddInstance` (`self.Instanced Chains`) (`KismetMathLibrary.MakeTransform` (`KismetMathLibrary.MakeVector` (* _index (`self.Chain Length`)))) false))
          (elif (< _returnvalue_4 _returnvalue_2)
            (for _index_2 (range _returnvalue_4 (+ _returnvalue_6 1))
              (`InstancedStaticMeshComponent.RemoveInstance` (`self.Instanced Chains`) _index_2))))))))

(fn `HandleSetHookShotStates`
  (params (`Hook States` :type "/Game/Grappling_Hook/E_Hookhot_States Enum" :default "NewEnumerator0"))
  (bind _output_get (set `self.Hook States` `Hook States`))
  (switch `/Game/Grappling_Hook/E_Hookhot_States` _output_get
    (:`NewEnumerator2`
      (`InstancedStaticMeshComponent.ClearInstances` (`self.Instanced Chains`)))))

(fn `UserConstructionScript`)