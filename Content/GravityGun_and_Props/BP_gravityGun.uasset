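; Gravity gun Blueprint that picks up, carries and drops physics-simulating objects.
; On trigger, a short visibility line trace from the Muzzle grabs any simulating component it hits through a PhysicsHandle and stores it as HeldComponent.
; Tick keeps the handle's target at a fixed distance in front of the Muzzle, and release lets go of the held component and clears the reference.
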(event `GravGunTrigger`
  (bind _muzzle (`self.Muzzle`))
  (bind _returnvalue (`SceneComponent.K2_GetComponentLocation` _muzzle))
  (bind (_outhit _returnvalue_2) (`KismetSystemLibrary.LineTraceSingle` :`Start` _returnvalue :`End` (+ _returnvalue (* (`SceneComponent.GetForwardVector` _muzzle) 300.0)) :`TraceChannel` "TraceTypeQuery1" :`DrawDebugType` "ForDuration"))
  (if _returnvalue_2
    (bind (_bblockinghit _binitialoverlap _time _distance _location _impactpoint _normal _impactnormal _physmat _hitactor _hitcomponent) (`GameplayStatics.BreakHitResult` _outhit))
    (if (`SceneComponent.IsSimulatingPhysics` _hitcomponent "None")
      (`PhysicsHandleComponent.GrabComponentAtLocation` (`self.PhysicsHandle`) _hitcomponent "None" (`SceneComponent.K2_GetComponentLocation` _hitcomponent))
      (set `self.HeldComponent` _hitcomponent)
      (`KismetSystemLibrary.PrintString` "Grab"))))

(event `GravGunRelease`
  (`self.HeldComponent`
    (:`then`
      (`PhysicsHandleComponent.ReleaseComponent` (`self.PhysicsHandle`))
      (`KismetSystemLibrary.PrintString` "Release")
      (set `self.HeldComponent` null))
    (:`else`)))

(event `self.ReceiveTick`
  (params (DeltaSeconds :type "Float (single-precision)"))
  (bind _muzzle (`self.Muzzle`))
  (`PhysicsHandleComponent.SetTargetLocation` (`self.PhysicsHandle`) (+ (`SceneComponent.K2_GetComponentLocation` _muzzle) (* (`SceneComponent.GetForwardVector` _muzzle) 100.0))))

(fn `UserConstructionScript`)