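; Player character Blueprint with dash, grapple and interaction, tuned from DataAssetPlayer on BeginPlay, which also spawns the rope and gravity gun.
; Tick line-traces BPI_Interactable actors for HUD prompts and sphere-traces for grapple targets.
; Left-click debug key fires the grapple: a second trace refines the target, then timelines extend the cable and pull the player in Flying mode.
; Dash briefly overrides velocity and friction with an FOV timeline and cooldown.
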(event Custom|Dash
  (bind _returnvalue (Class|Pawn|GetLastMovementInputVector))
  (bind _charactermovement (Variables|Character|GetCharacterMovement))
  (bind _charactermovement_2 (Variables|Character|GetCharacterMovement))
  (bind _dash_distance (Variables|Dash|GetDash_Distance))
  (bind _returnvalue_2 (* _dash_distance 1e+01))
  ;[1 0.05 0.05] Dash
  (if (Variables|Dash|GetCan_Dash)
    (Variables|Dash|SetCan_Dash false)
    (Variables|Dash|SetIs_Dashing true)
    (Variables|Dash|SetOld_Velocity (Variables|/Script/Engine.MovementComponent|GetVelocity _charactermovement))
    (Variables|Dash|SetOld_Ground_Friction (Variables|/Script/Engine.CharacterMovementComponent|GetGroundFriction _charactermovement))
    (Variables|/Script/Engine.CharacterMovementComponent|SetGroundFriction _charactermovement 0.0)
    (if (Math|Vector|VectorIsNearlyZero _returnvalue)
      (Variables|/Script/Engine.MovementComponent|SetVelocity _charactermovement (* (Transformation|GetActorForwardVector) _returnvalue_2))
      (else
        (Variables|/Script/Engine.MovementComponent|SetVelocity _charactermovement (* (Math|Vector|Normalize _returnvalue) _returnvalue_2))))
    (CallFunction|StartFOV)
    (Utilities|FlowControl|Delay (Variables|Dash|GetDash_Duration))
    (CallFunction|StopFOV)
    (Variables|Dash|SetIs_Dashing false)
    (Variables|/Script/Engine.CharacterMovementComponent|SetGroundFriction _charactermovement_2 (Variables|Dash|GetOld_Ground_Friction))
    (Variables|/Script/Engine.MovementComponent|SetVelocity _charactermovement_2 (Variables|Dash|GetOld_Velocity))
    (Utilities|FlowControl|Delay (Variables|Dash|GetDash_Cooldown))
    (Variables|Dash|SetCan_Dash true)))

(event Custom|Grapple
  (bind _returnvalue (Transformation|GetActorRotation))
  ;[1 0.17 0] Grapple Cable & Target Lock
  (if (and (not (Variables|Grapple|GetIs_Grappling)) (Variables|Grapple|GetDid_Grapple_Hit))
    (if (Variables|Grapple|GetIs%20Grapple%20Ledge)
      (if (Grapple|GetGrappleTargetInfo)
        (if (not (<= (Variables|Grapple|GetGrapple%20Distance) (Variables|Data|Grapple|GetMin%20Grapple%20Distance)))
          (Variables|/Script/CableComponent.CableComponent|SetbAttachStart (Variables|/Game/Grappling_Hook/BP_GrappleRope.BP_GrappleRope_C|GetCable (Variables|References|GetGrapple_Cable_Ref)) true)
          ;;[0.15 0.15 0.15 0.5] For ABP
          (Variables|Grapple|SetIs_Grappling true)
          (Transformation|SetActorRotation (Math|Rotator|MakeRotator (.roll _returnvalue) (.pitch _returnvalue) (.yaw (Variables|Grapple|GetGrapple%20Target%20Rotation))))
          (Variables|Grapple|SetCurrent%20Actor%20Loaction (Transformation|GetActorLocation))
          (Variables|/Script/Engine.CharacterMovementComponent|SetGravityScale (Variables|Character|GetCharacterMovement) 0.5)
          (bind _alpha (Timeline|T_Grapple_Move_Cable PlayFromStart)
            (:Update
              (Grapple|GrappleSetCableLocation _alpha))
            (:Finished
              (CallFunction|StartGrappling))))))))

(event Custom|Start%20Grappling
  (bind _charactermovement (Variables|Character|GetCharacterMovement))
  ;[1 0.17 0] Start Grappling
  (Pawn|Components|CharacterMovement|SetMovementMode _charactermovement "MOVE_Flying" 0)
  (Components|Movement|StopMovementImmediately _charactermovement)
  (Variables|Grapple|SetCurrent%20Actor%20Loaction (Transformation|GetActorLocation))
  (Grapple|GrappleCalcPlayerGrappleTargetLocation)
  (bind _alpha (Timeline|T_GrappleMoveActor PlayFromStart)
    (:Update
      (Grapple|GrappleSetPlayerLocation _alpha))
    (:Finished
      (CallFunction|EndGrappling))))

(event Custom|Stop%20Grappling
  (bind _charactermovement (Variables|Character|GetCharacterMovement))
  ;[1 0.17 0] Grappling (Timeline Event)
  (Pawn|Components|CharacterMovement|SetMovementMode _charactermovement "MOVE_Falling" 0)
  (Variables|Grapple|SetIs_Grappling false)
  (Variables|/Script/Engine.CharacterMovementComponent|SetGravityScale _charactermovement 1.75))

(event Custom|Start%20FOV
  ;[0 1 1] FOV Change
  (if (not (Variables|FOV|GetHas_Applied_FOV))
    (Variables|FOV|SetHas_Applied_FOV true)
    (Variables|FOV|SetOld_FOV (Variables|/Script/Engine.CameraComponent|GetFieldOfView (Variables|Default|GetCamera)))
    (bind (_direction _fov_alpha) (Timeline|T_FOV Play)
      (:Update
        (Camera|SetFieldOfView (Variables|Default|GetCamera) (Math|Float|Lerp (Variables|FOV|GetOld_FOV) (Variables|FOV|GetDash_Fov) _fov_alpha)))
      (:Finished
        (if (Utilities|Enum|Equal(Enum) _direction "Backward")
          (Variables|FOV|SetHas_Applied_FOV false))))))

(event Custom|End%20Grappling
  ;[1 0.17 0] End Grappling (Anim Transition Event)
  (CallFunction|StopGrappling)
  (Variables|/Script/CableComponent.CableComponent|SetbAttachStart (Variables|/Game/Grappling_Hook/BP_GrappleRope.BP_GrappleRope_C|GetCable (Variables|References|GetGrapple_Cable_Ref)) false)
  (Variables|Grapple|SetIs_Grappling false)
  (Variables|/Script/Engine.CharacterMovementComponent|SetGravityScale (Variables|Character|GetCharacterMovement) (Variables|/Game/_Manager/Data/3C/PDA_Player.PDA_Player_C|GetGravity (Variables|References|GetData_Asset_Player))))

(event Custom|Stop%20FOV
  ;[0 1 1] FOV Change
  (if (Variables|FOV|GetHas_Applied_FOV)
    (bind (_direction _fov_alpha) (Timeline|T_FOV Reverse)
      (:Update
        (Camera|SetFieldOfView (Variables|Default|GetCamera) (Math|Float|Lerp (Variables|FOV|GetOld_FOV) (Variables|FOV|GetDash_Fov) _fov_alpha)))
      (:Finished
        (if (Utilities|Enum|Equal(Enum) _direction "Backward")
          (Variables|FOV|SetHas_Applied_FOV false))))))

(event Input|EnhancedActionEvents|EnhancedInputActionIA_Interact
  (params (ActionValue :type Boolean) (ElapsedSeconds :type Float%20%28double-precision%29) (TriggeredSeconds :type Float%20%28double-precision%29) (InputAction :type Input%20Action%20Object%20Reference :default "/Game/_Manager/Input/Actions/IA_Interact.IA_Interact"))
  (:Started
    (Interaction|OnInteract)))

(event EventBeginPlay
  (bind _aspc_player (Utilities|Casting|CastToPC_Player (Pawn|GetController)))
  (Variables|References|SetPlayer_Controller_Ref _aspc_player)
  (CallFunction|SetupPlayerFeeling)
  (bind _returnvalue (Game|SpawnActorfromClass "/Game/Grappling_Hook/BP_GrappleRope.BP_GrappleRope_C" (Transformation|GetActorTransform) "Undefined" "MultiplyWithRoot" 0 "hand_r" 0))
  (Variables|References|SetGrapple_Cable_Ref _returnvalue)
  (bind _returnvalue_2 (Game|SpawnActorfromClass "/Game/GravityGun_and_Props/BP_gravityGun.BP_gravityGun_C" (Math|Transform|MakeTransform "0, 0, 0" "0, 0, 0" "1.000000,1.000000,1.000000") "Undefined" "MultiplyWithRoot" 0 0))
  (bind _output_get (Variables|Default|SetGravityGun _returnvalue_2))
  (Transformation|AttachComponentToComponent _output_get (Variables|Default|GetGravGunAttach) "None" "SnapToTarget" "SnapToTarget" "SnapToTarget" true))

(event EventTick
  (params (DeltaSeconds :type Float%20%28single-precision%29))
  (bind (_start _end) (|GrappleTransformCalculations))
  (Utilities|FlowControl|Sequence
    (:then_0
      (Interaction|InteractSetText))
    (:then_1
      (if (not (Variables|Grapple|GetIs_Grappling))
        (bind (_outhit _returnvalue) (Collision|SphereTraceByChannel _start _end 366.0 "TraceTypeQuery1" false 0 "ForOneFrame"))
        (bind _output_get (Variables|Grapple|SetDid_Grapple_Hit _returnvalue))
        (if _output_get
          (bind _output_get_2 (Variables|Grapple|SetGrapple%20Out%20Hit _outhit))
          (Rendering|Debug|DrawDebugPoint (.ImpactPoint (Collision|BreakHitResult _output_get_2)) 25.0 "(R=1.000000,G=1.000000,B=1.000000,A=1.000000)" 0.0))))))

(event Input|MouseEvents|DebugKeyLeftMouseButton
  (params (Key :type Key%20Structure :default "None") (ActionValue :type Input%20Action%20Value%20Structure))
  (:Pressed
    (CallFunction|Grapple)))

(fn ConstructionScript)

(fn SetupPlayerFeeling
  (bind _returnvalue (Game|GetPlayerCameraManager 0))
  (bind _charactermovement (Variables|Character|GetCharacterMovement))
  (bind _data_asset_player (Variables|References|GetData_Asset_Player))
  (bind _data_asset_player_2 (Variables|References|GetData_Asset_Player))
  (bind _data_asset_player_3 (Variables|References|GetData_Asset_Player))
  (Utilities|FlowControl|Sequence
    (:then_0
      (Variables|Data|State|SetPlayer_State (Variables|/Game/_Manager/Data/3C/PDA_Player.PDA_Player_C|GetPlayer_State _data_asset_player_3))
      (bind _output_get (Variables|Health|SetMax_HP (Variables|/Game/_Manager/Data/3C/PDA_Player.PDA_Player_C|GetMax_HP _data_asset_player_3)))
      (Variables|Health|SetCurrent_HP _output_get)
      (bind _output_get_2 (Variables|Data|Camera|SetCurrent_Fov (Variables|/Game/_Manager/Data/3C/PDA_Player.PDA_Player_C|GetCurrent_FOV _data_asset_player_3)))
      (Camera|SetFieldOfView (Variables|Default|GetCamera) _output_get_2)
      (bind _output_get_3 (Variables|/Script/Engine.CharacterMovementComponent|SetMaxWalkSpeed _charactermovement (Variables|/Game/_Manager/Data/3C/PDA_Player.PDA_Player_C|GetWalk_Speed _data_asset_player_3)))
      (Variables|Data|Movement|SetMax_Walk_Speed%20 _output_get_3)
      (Variables|Data|Movement|SetRun_Speed (Variables|/Game/_Manager/Data/3C/PDA_Player.PDA_Player_C|GetRun_Speed _data_asset_player_3))
      (Variables|/Script/Engine.CharacterMovementComponent|SetGravityScale _charactermovement (Variables|/Game/_Manager/Data/3C/PDA_Player.PDA_Player_C|GetGravity _data_asset_player_3))
      (Variables|/Script/Engine.CharacterMovementComponent|SetJumpZVelocity _charactermovement (Variables|/Game/_Manager/Data/3C/PDA_Player.PDA_Player_C|GetJump_Height _data_asset_player_3))
      (Variables|/Script/Engine.CharacterMovementComponent|SetAirControl _charactermovement (Variables|/Game/_Manager/Data/3C/PDA_Player.PDA_Player_C|GetAir_Control _data_asset_player_3)))
    (:then_1
      (Variables|Dash|SetDash_Distance (Variables|/Game/_Manager/Data/3C/PDA_Player.PDA_Player_C|GetDash_Distance _data_asset_player))
      (Variables|FOV|SetDash_Fov (Variables|/Game/_Manager/Data/3C/PDA_Player.PDA_Player_C|GetDash_FOV _data_asset_player))
      (Variables|Dash|SetDash_Duration (Variables|/Game/_Manager/Data/3C/PDA_Player.PDA_Player_C|GetDash_Duration _data_asset_player))
      (Variables|Dash|SetDash_Cooldown (Variables|/Game/_Manager/Data/3C/PDA_Player.PDA_Player_C|GetDash_Cooldown _data_asset_player)))
    (:then_2
      (Variables|Data|Camera|SetCamera_Invert (Variables|/Game/_Manager/Data/3C/PDA_Player.PDA_Player_C|GetCamera_Invert _data_asset_player))
      (Variables|Data|Camera|SetCamera_Horizontal_Speed (Variables|/Game/_Manager/Data/3C/PDA_Player.PDA_Player_C|GetCamera_Horizontal_Speed _data_asset_player))
      (Variables|Data|Camera|SetCamera_Vertical_Speed (Variables|/Game/_Manager/Data/3C/PDA_Player.PDA_Player_C|GetCamera_Vertical_Speed _data_asset_player))
      (bind _output_get_4 (Variables|Data|Camera|SetCamera_View_Pitch_Min (Variables|/Game/_Manager/Data/3C/PDA_Player.PDA_Player_C|GetCamera_View_Pitch_Min _data_asset_player)))
      (Variables|/Script/Engine.PlayerCameraManager|SetViewPitchMin _returnvalue _output_get_4)
      (bind _output_get_5 (Variables|Data|Camera|SetCamera_View_Pitch_Max (Variables|/Game/_Manager/Data/3C/PDA_Player.PDA_Player_C|GetCamera_View_Pitch_Max _data_asset_player)))
      (Variables|/Script/Engine.PlayerCameraManager|SetViewPitchMax _returnvalue _output_get_5))
    (:then_3
      (bind _output_get_6 (Variables|Energy|SetMax_Energy (Variables|/Game/_Manager/Data/3C/PDA_Player.PDA_Player_C|GetMax_Energy _data_asset_player_2)))
      (Variables|Energy|SetEnergy _output_get_6)
      (Variables|Data|Movement|SetIs_Sprint_Toggle (Variables|/Game/_Manager/Data/3C/PDA_Player.PDA_Player_C|GetIs_Sprint_Toggle _data_asset_player_2))
      (Variables|Data|Interaction|SetInteraction_Range (Variables|/Game/_Manager/Data/3C/PDA_Player.PDA_Player_C|GetInteraction_Range _data_asset_player_2))
      (Variables|Data|Grapple|SetMin%20Grapple%20Distance (Variables|/Game/_Manager/Data/3C/PDA_Player.PDA_Player_C|GetGrapple%20Min%20Distance _data_asset_player_2)))))

(fn ConsumeEnergy
  (params (Energy%20to%20Remove :type Integer))
  (if (<= Energy%20to%20Remove (Variables|Energy|GetEnergy))
    (Variables|Energy|SetEnergy (- (Variables|Energy|GetEnergy) Energy%20to%20Remove))
    (return true)
    (else
      (return false))))

(fn RestoreEnergy
  (params (Amount%20to%20Restore :type Integer))
  (Variables|Energy|SetEnergy (+ (Variables|Energy|GetEnergy) Amount%20to%20Restore)))

(fn InteractTrace
  (bind _capsulecomponent (Variables|Collision|GetCapsuleComponent))
  (bind _returnvalue (Transformation|GetWorldLocation _capsulecomponent))
  (bind _returnvalue_2 (+ _returnvalue "0.000000,0.000000,20.000000"))
  (bind _outhit (Collision|LineTraceByChannel _returnvalue_2 (+ _returnvalue_2 (* (Math|Vector|GetForwardVector (Variables|Default|GetCamera)) (Variables|Data|Interaction|GetInteraction_Range))) "TraceTypeQuery1" false (Utilities|Array|MakeArray self) "None"))
  (if (Utilities|DoesObjectImplementInterface (.hitactor _outhit) "/Game/HelioBloom/BP_Interface/BPI_Interactable.BPI_Interactable_C")
    (Variables|Interaction|SetInteract_Hit_Actor (.hitactor _outhit))
    (bind _can_interact (Class|BPIInteractable|CanInteract(Message) (Variables|Interaction|GetInteract_Hit_Actor)))
    (if _can_interact
      (bind _foundwidgets (Widget|GetAllWidgetsOfClass "/Game/HelioBloom/UI/WBP_PlayerHUD.WBP_PlayerHUD_C" true))
      (Variables|Interaction|SetHUD_Ref (Utilities|Array|Get(acopy) _foundwidgets))
      (bind (_type _text _cost_energy) (Class|BPIInteractable|IsInteractable/GetDetails(Message) (Variables|Interaction|GetInteract_Hit_Actor)))
      (Utilities|FlowControl|Sequence
        (:then_0
          (Variables|Interaction|SetInteract_Text _text)
          (Variables|Interaction|SetInteract_Energy _cost_energy))
        (:then_1
          (Variables|Interaction|SetInteracting true)
          (return _type))))
    (elif (Variables|Interaction|GetInteracting)
      (bind _foundwidgets_2 (Widget|GetAllWidgetsOfClass "/Game/HelioBloom/UI/WBP_PlayerHUD.WBP_PlayerHUD_C" true))
      (bind _output_get (Variables|Interaction|SetHUD_Ref (Utilities|Array|Get(acopy) _foundwidgets_2)))
      (Variables|/Script/UMG.TextBlock|SetText (Variables|/Game/HelioBloom/UI/WBP_PlayerHUD.WBP_PlayerHUD_C|GetInteraction_Text _output_get) "")
      (Variables|Interaction|SetInteracting false))))

(fn InteractSetText
  (bind _type (Interaction|InteractTrace))
  (switch Utilities|FlowControl|Switch|SwitchonE_Interact _type
    (:NewEnumerator2
      (bind _can_interact (Class|BPIInteractable|CanInteract(Message) (Variables|Interaction|GetInteract_Hit_Actor)))
      (if _can_interact
        (Variables|/Script/UMG.TextBlock|SetText (Variables|/Game/HelioBloom/UI/WBP_PlayerHUD.WBP_PlayerHUD_C|GetInteraction_Text (Variables|Interaction|GetHUD_Ref)) (Utilities|Text|FormatText "Press E or (X) to {Text}" (Variables|Interaction|GetInteract_Text)))))))

(fn OnInteract
  (bind _type (Interaction|InteractTrace))
  (switch Utilities|FlowControl|Switch|SwitchonE_Interact _type
    (:NewEnumerator2
      (Class|BPIInteractable|OnInteract(Message) (Variables|Interaction|GetInteract_Hit_Actor)))))

(fn GetGrappleTargetInfo
  (bind _grapple_out_hit (Variables|Grapple|GetGrapple%20Out%20Hit))
  (bind _impactpoint (Collision|BreakHitResult _grapple_out_hit))
  (bind (_outhit _returnvalue) (Collision|SphereTraceForObjects (+ _impactpoint "0.000000,0.000000,33.000000") (+ _impactpoint "0.000000,0.000000,-33.000000") 33.0 (Utilities|Array|MakeArray "ObjectTypeQuery1") false 0 "None"))
  (if _returnvalue
    (bind _output_get (Variables|Grapple|SetSecond%20Grapple%20Out%20Hit _outhit))
    (Grapple|GrappleGetTargetTransform _output_get)
    (return _returnvalue)))

(fn GrappleGetTargetTransform
  (params (Second%20Out%20Hit :type Hit%20Result%20Structure))
  (bind _returnvalue (Transformation|GetActorLocation))
  (bind _output_get (Variables|Grapple|SetGrapple%20Target%20Location (.ImpactPoint (Collision|BreakHitResult Second%20Out%20Hit))))
  (Variables|Grapple|SetGrapple%20Target%20Rotation (Math|Rotator|FindLookatRotation _returnvalue _output_get))
  (Variables|Grapple|SetGrapple%20Distance (Math|Vector|Distance(Vector) _output_get _returnvalue))
  (return))

(fn GrappleCalcPlayerGrappleTargetLocation
  (Variables|Grapple|SetGrapple%20Target%20Location (+ (* (Transformation|GetActorForwardVector) -111.0) (.ImpactPoint (Collision|BreakHitResult (Variables|Grapple|GetSecond%20Grapple%20Out%20Hit)))))
  (return))

(fn GrappleSetCableLocation
  (params (Alpha :type Float%20%28double-precision%29))
  (Transformation|SetActorLocation (Variables|References|GetGrapple_Cable_Ref) (Math|Vector|Lerp(Vector) (Transformation|GetActorLocation) (+ (Variables|Grapple|GetGrapple%20Target%20Location) "0.0,0.0,-5.0") Alpha) false false))

(fn GrappleSetPlayerLocation
  (params (Alpha :type Float%20%28double-precision%29))
  (Transformation|SetActorLocation (Math|Vector|Lerp(Vector) (Transformation|GetActorLocation) (+ (Variables|Grapple|GetGrapple%20Target%20Location) "0.0,0.0,-5.0") Alpha) true false))