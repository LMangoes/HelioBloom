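; Laser emitter actor that fires a beam along its Arrow component every tick, bouncing it off mirrors.
; ShootLaser runs a fixed-range line trace against a single object type from the arrow's location.
; On a hit it draws a red debug line to the impact point and, if the actor is a BP_Mirror, calls ReflectLaser with the trace start.
; The beam is visualised only through debug drawing.
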(event `self.ReceiveTick`
  (params (DeltaSeconds :type "Float (single-precision)"))
  (`self.ShootLaser` (`SceneComponent.GetForwardVector` (`self.Arrow`))))

(event `ShootLaser`
  (params (Direction :type "Vector Structure"))
  (bind _returnvalue (`SceneComponent.K2_GetComponentLocation` (`self.Arrow`)))
  (bind (_outhit _returnvalue_2) (`KismetSystemLibrary.LineTraceSingleForObjects` :`Start` _returnvalue :`End` (+ _returnvalue (* Direction 1000.0)) :`ObjectTypes` (`|MakeArray` "ObjectTypeQuery8" :!type "EObjectTypeQuery Enum") :`DrawDebugType` "ForDuration"))
  (if _returnvalue_2
    (bind (_bblockinghit _binitialoverlap _time _distance _location _impactpoint _normal _impactnormal _physmat _hitactor _hitcomponent _hitbonename _bonename _hititem _elementindex _faceindex _tracestart) (`GameplayStatics.BreakHitResult` _outhit))
    (`KismetSystemLibrary.DrawDebugLine` _tracestart _impactpoint (struct :`R` 1.0 :`A` 1.0) 1.0 3.0)
    (bind _asbp_mirror (cast `/Game/Lasers_Mirrors/BP_Mirror` _hitactor))
    (`/Game/Lasers_Mirrors/BP_Mirror.ReflectLaser` _asbp_mirror _tracestart)))

(fn `UserConstructionScript`)