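; BP_Mirror is a mirror actor that redirects an incoming laser.
; ReflectLaser takes the laser source position and finds its angle to the Arrow component's forward vector with a dot product and arccosine.
; It rotates that forward vector around world Z by the angle and passes the result to ShootLaser.
; The angle is unsigned, so the rotation always turns the same way, whichever side the source is on.
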(event `ReflectLaser`
  (params (`Laser Source` :type "Vector Structure"))
  (`self.ShootLaser` (`KismetMathLibrary.RotateAngleAxis` (`SceneComponent.GetForwardVector` (`self.Arrow`)) (`KismetMathLibrary.DegAcos` (`KismetMathLibrary.Dot_VectorVector` (`KismetMathLibrary.Normal` (- `Laser Source` (`self.K2_GetActorLocation`))) (`SceneComponent.GetForwardVector` (`self.Arrow`)))) (0.0 0.0 1.0))))

(fn `UserConstructionScript`)