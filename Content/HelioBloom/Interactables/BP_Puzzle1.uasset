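; BP_Puzzle1 is an interactable rotating puzzle piece that is valid when its rotation index matches the correct index.
; BeginPlay applies a random quarter-turn yaw, and each interaction turns it another 90 degrees, cycling the index through four states.
; Tick updates the Validate flag every frame and prints the result as debug text.
; The construction script picks the cube's material from an array, while interface functions report interactability, prompt text and energy cost.
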(event `self.ReceiveBeginPlay`
  ;[1 0 0.8904 0.5] Random Rotation Spawn
  (bind _output_get (set `self.Rotation Index` (`KismetMathLibrary.RandomIntegerInRange` 1 4)))
  (`SceneComponent.K2_AddWorldRotation` (`self.DefaultSceneRoot`) (`KismetMathLibrary.MakeRotator` 0.0 0.0 (* _output_get 90)) false false))

(event `self.ReceiveTick`
  (params (DeltaSeconds :type "Float (single-precision)"))
  (if (== (`self.Rotation Index`) (`self.Correct_Index`))
    (set `self.Validate` true)
    (`KismetSystemLibrary.PrintString` "Correct" true true (struct :`R` 0.012363 :`G` 1.0 :`B` 0.328208 :`A` 1.0) 0.0)
    (else
      (set `self.Validate` false)
      (`KismetSystemLibrary.PrintString` "Wrong" true true (struct :`R` 1.0 :`G` 0.043221 :`A` 1.0) 0.0))))

(event `self.On_Interact`
  (`SceneComponent.K2_AddWorldRotation` (`self.DefaultSceneRoot`) (`KismetMathLibrary.MakeRotator` 0.0 0.0 90.0) false false)
  (if (not (== (`self.Rotation Index`) 4))
    (`/Engine/EditorBlueprintResources/StandardMacros.IncrementInt` (`self.Rotation Index`))
    (else
      (set `self.Rotation Index` 1))))

(fn `Can_Interact`
  (returns (Can_Interact :type Boolean))
  (return (`self.Can Interact`)))

(fn `Is Interactable / Get Details`
  (returns (Type :type "/Game/HelioBloom/Enums/E_Interact Enum") (Text :type Text) (`Cost Energy` :type Integer))
  (return "NewEnumerator2" (`self.Text`) (`self.Cost Energy`)))

(fn `UserConstructionScript`
  (`PrimitiveComponent.SetMaterial` (`self.Cube`) 0 (`|GetArrayItem` (`self.Material_Array `) (`self.Texture_Index`))))